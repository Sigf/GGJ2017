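; Player Blueprint that runs automatically along world +Y and glides vertically between evenly spaced height levels.
; Each tick feeds delta-scaled RunningSpeed into CharacterMovement as input, then lerps actor Z toward CurrentLevel's share of MaxHeight divided by LevelCounts.
; The lerp alpha is VerticalSpeed times delta time, clamped to one, giving an eased approach applied through an unswept SetActorLocation.
; Nothing in these graphs changes CurrentLevel.
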(event `self.ReceiveTick`
  (params (DeltaSeconds :type "Float (single-precision)"))
  (`self.Move Right` DeltaSeconds)
  (`self.Lerp To Level`))

(fn `Lerp To Level`
  (`self.K2_SetActorLocation` (`KismetMathLibrary.MakeVector` (.x (`self.K2_GetActorLocation`)) (.y (`self.K2_GetActorLocation`)) (`KismetMathLibrary.Lerp` (.z (`self.K2_GetActorLocation`)) (* (/ (`self.Max Height`) (`KismetMathLibrary.Conv_IntToDouble` (`self.LevelCounts`))) (`KismetMathLibrary.Conv_IntToDouble` (`self.CurrentLevel`))) (`KismetMathLibrary.FClamp` (* (`self.Vertical Speed`) (`GameplayStatics.GetWorldDeltaSeconds`)))))))

(fn `Move Right`
  (params (Delta :type "Float (double-precision)"))
  (`PawnMovementComponent.AddInputVector` (`self.CharacterMovement`) (* (0.0 1.0 0.0) (* (`self.Running Speed`) Delta)) false))

(fn `UserConstructionScript`)